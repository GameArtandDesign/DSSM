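; Parent Blueprint for Paper2D spawnables that are either collectibles or hazards, resolved on touching the player or the ground.
; Overlapping a living player adds score for collectibles or costs health otherwise, calling GameOver below 1 health.
; Tick updates the flipbook and checks a Y threshold as ground, where missed collectibles cost health.
; Either contact triggers a Disappear flipbook and short lifespan; movement and ground-touch functions are empty stubs.
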(event EventBeginPlay
  (bind _returnvalue (Actor|GetActorOfClass "/Game/Blueprints/BP_GameStateBase.BP_GameStateBase_C"))
  (Variables|Default|SetGameStateBase%20Ref _returnvalue))

(event Collision|EventActorBeginOverlap
  (params (OtherActor :type Actor%20Object%20Reference))
  (bind _player_ref (Variables|Default|GetPlayer%20Ref))
  ;[1 1 1] If Touching Player
  (bind _asbp_player_character (Utilities|Casting|CastToBP_PlayerCharacter OtherActor))
  ;[1 1 1] If Player has > 0 Health
  (if (> (Variables|/Game/Blueprints/BP_PlayerCharacter.BP_PlayerCharacter_C|GetHealth _asbp_player_character) 0)
    ;[1 1 1] If hasn't been collected (or touched) already
    (if (not (Variables|GameplayBools|GetCollected))
      (Variables|GameplayBools|SetCollected true)
      (if (Variables|GameplayBools|GetIsCollectible?)
        (CollisionEvents|TouchingPlayerGood (Variables|Default|GetScore%20to%20Add))
        (Variables|/Game/Blueprints/BP_PlayerCharacter.BP_PlayerCharacter_C|SetScore _player_ref (+ (Variables|/Game/Blueprints/BP_PlayerCharacter.BP_PlayerCharacter_C|GetScore _player_ref) (Variables|Default|GetScore%20to%20Add)))
        (else
          (CollisionEvents|LoseLife)))
      (CallFunction|Disappear))))

(event EventTick
  (params (DeltaSeconds :type Float%20%28single-precision%29))
  (bind _time_to_disappear_ (CallFunction|GroundCheck))
  (if _time_to_disappear_
    (CallFunction|Disappear)))

(fn ConstructionScript
  (Variables|Default|SetThe%20GameState (Game|GetGameState))
  (bind _returnvalue (Actor|GetActorOfClass "/Game/Blueprints/BP_PlayerCharacter.BP_PlayerCharacter_C"))
  (Variables|Default|SetPlayer%20Ref _returnvalue))

(fn TouchingPlayerGood
  (params (AddScorePoint :type Integer))
  (Variables|Default|SetScore%20to%20Add (+ AddScorePoint (Variables|Default|GetScore%20to%20Add))))

(fn LoseLife
  (bind _player_ref (Variables|Default|GetPlayer%20Ref))
  (bind _output_get (Variables|/Game/Blueprints/BP_PlayerCharacter.BP_PlayerCharacter_C|SetHealth _player_ref (- (Variables|/Game/Blueprints/BP_PlayerCharacter.BP_PlayerCharacter_C|GetHealth _player_ref) (Variables|Default|GetLife%20to%20Subtract))))
  (if (< _output_get 1)
    (bind _asbp_game_state_base (Utilities|Casting|CastToBP_GameStateBase (Game|GetGameState)))
    (Default|GameOver _asbp_game_state_base)))

(fn TouchingGroundGood)

(fn TouchingGroundBad
  (params (NewParam :type Integer)))

(fn TouchingPlayerCall
  (if (Variables|GameplayBools|GetIsCollectible?)
    ;[1 1 1] Will be overridden in Children, default to add score/subtract life
    (CollisionEvents|TouchingPlayerGood)
    (else
      (CollisionEvents|LoseLife)))
  (Actor|SetLifeSpan 1.0))

(fn TouchingGroundCall
  (if (Variables|GameplayBools|GetIsCollectible?)
    ;[1 1 1] To be Overridden in Children. Default to Lose Life/Nothing
    (CollisionEvents|TouchingGroundBad)
    (else
      (CollisionEvents|TouchingGroundGood)))
  (Actor|SetLifeSpan 1.0))

(fn UpdateFlipbook
  ;[1 1 1] Called every tick. Values passed elsewhere
  (Sprite|SetFlipbook (Variables|Default|GetPaperFlipbook) (Utilities|Select :Index (Variables|Default|GetSpawnable%20FB) :NewEnumerator0 (Variables|Default|GetIdle%20FB) :NewEnumerator1 (Variables|Default|GetDisappear%20FB))))

(fn Movement
  (params (Spawn%20Over? :type Boolean)))

(fn GroundCheck
  (CallFunction|UpdateFlipbook)
  ;[1 1 1] Check if "on ground" every tick
  (if (and (>= (.y (Transformation|GetActorLocation)) 775.0) (not (Variables|GameplayBools|GetCollected)))
    (Variables|GameplayBools|SetCollected true)
    (Variables|GameplayBools|SetOn%20Ground? true)
    ;[1 1 1] Do Touching Ground functionality
    (if (Variables|GameplayBools|GetIsCollectible?)
      (CollisionEvents|LoseLife))
    (return true)
    (else
      (return false))))

(fn Disappear
  ;[1 1 1] Play Disappear FB and Destroy Actor, regardless of Good/Bad collision
  (Variables|Default|SetSpawnable%20FB "NewEnumerator1")
  (Variables|GameplayBools|SetCollected true)
  (Actor|SetLifeSpan 0.2))