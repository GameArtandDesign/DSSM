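; BP_SpawnBox is the animated squirrel spawner that throws acorns, nuggets and tree branches while the player has health.
; A looping timer plus a random delay calls ThrowSpawnable, using arrays indexed by TimerSpeedIndex for timing and item range.
; Every fifth acorn raises that index, fall speed and player speed.
; Tick updates the flipbook, while Movement steps to random points in a same-frame loop and reschedules itself.
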(event Custom|CallThrowSpawnable
  ;[1 1 1] Called by BeginPlay timer, then delayed before ThrowSpawnable
  (Variables|Default|SetFBSelect "NewEnumerator0")
  (Utilities|FlowControl|Delay (Math|Random|RandomFloatinRange (Utilities|Array|Get(acopy) (Variables|Default|GetMinTimerArray) (Variables|Default|GetTimer%20Speed%20Index)) (Utilities|Array|Get(acopy) (Variables|Default|GetMaxTimerArray) (Variables|Default|GetTimer%20Speed%20Index))))
  (if (> (Variables|/Game/Blueprints/BP_PlayerCharacter.BP_PlayerCharacter_C|GetHealth (Variables|Default|GetPlayer%20Ref)) 0)
    (CallFunction|ThrowSpawnable)
    (if true
      (Utilities|FlowControl|Delay 1.3)
      (Variables|Default|SetFBSelect "NewEnumerator2"))
    (else
      (Variables|Default|SetFBSelect "NewEnumerator4"))))

(event Custom|Increase%20Speed
  (bind _player_ref (Variables|Default|GetPlayer%20Ref))
  ;[1 1 1] Increase how fast Acorns fall (some, not much)
  (bind _output_get (Variables|Default|SetGlobal%20Speed (+ (Variables|Default|GetGlobal%20Speed) 0.2)))
  (Development|PrintString (Utilities|String|ToString(Float) _output_get) true true "(R=0.008018,G=1.000000,B=0.097723,A=1.000000)")
  (Utilities|FlowControl|Sequence
    (:then_0
      ;[1 1 1] Decrease how much time there can be between Throw Spawnable calls, if not at the max Index (size of Min/MaxTimerArray)
      (if (<= (Variables|Default|GetTimer%20Speed%20Index) (Utilities|Array|Length (Variables|Default|GetMaxTimerArray)))
        (bind _output_get_2 (Variables|Default|SetTimer%20Speed%20Index (+ (Variables|Default|GetTimer%20Speed%20Index) 1)))
        ;[1 1 1] Marginally increment Player Speed. Want this to be fair, but not noticeable.
        (Development|PrintString (Utilities|String|ToString(Integer) _output_get_2) true true "(R=0.032042,G=0.952232,B=1.000000,A=1.000000)")
        (Variables|/Game/Blueprints/BP_PlayerCharacter.BP_PlayerCharacter_C|SetPlayerSpeed _player_ref (+ (Variables|/Game/Blueprints/BP_PlayerCharacter.BP_PlayerCharacter_C|GetPlayerSpeed _player_ref) 0.02))
        (else
          (bind _output_get_3 (Variables|Default|SetGlobal%20Speed (+ (Variables|Default|GetGlobal%20Speed) 0.1)))
          (Development|PrintString (Utilities|String|ToString(Float) _output_get_3) true true "(R=0.008018,G=1.000000,B=0.097723,A=1.000000)"))))
    (:then_1
      ;[1 1 1] Start moving SpawnBox left and right once TSI > 6
      (if (> (Variables|Default|GetTimer%20Speed%20Index) 6)
        _))))

(event EventBeginPlay
  ;[1 1 1] Reset to Starting Location (relevant if moved)
  (Transformation|SetActorLocation (Variables|Default|GetStarting%20Location) false true)
  ;[1 1 1] Call ThrowSpawnable every min-max seconds
  (Utilities|Time|SetTimerbyEvent (delegate Custom|CallThrowSpawnable) 1.0 true 1.4)
  ;[1 1 1] Initialize Variables
  (Variables|Default|SetGlobal%20Speed (Variables|Default|GetStarting%20Speed))
  (Variables|Default|SetTimer%20Speed%20Index 0)
  (Variables|Default|SetAcorns%20Thrown%20Count 0)
  ;[1 1 1] Start moving SpawnBox left and right once TSI > 6
  (Utilities|FlowControl|DoOnce false ; enters at Reset
    (:Completed
      (CallFunction|Movement) ; Logic calls itself
    )))

(event EventTick
  (params (DeltaSeconds :type Float%20%28single-precision%29))
  (CallFunction|UpdateAnimation)
  (Variables|Default|SetLocal%20Health (Variables|/Game/Blueprints/BP_PlayerCharacter.BP_PlayerCharacter_C|GetHealth (Variables|Default|GetPlayer%20Ref)))
  (if (not (> (Variables|/Game/Blueprints/BP_PlayerCharacter.BP_PlayerCharacter_C|GetHealth (Variables|Default|GetPlayer%20Ref)) 0))
    (Variables|Default|SetFBSelect "NewEnumerator4")))

(fn ConstructionScript
  (Variables|Default|SetTheGameState (Game|GetGameState))
  (Variables|Default|SetFBSelect "NewEnumerator2")
  (bind _returnvalue (Actor|GetActorOfClass "/Game/Blueprints/BP_PlayerCharacter.BP_PlayerCharacter_C"))
  (Variables|Default|SetPlayer%20Ref _returnvalue))

(fn ThrowSpawnable
  (bind _returnvalue (Transformation|GetActorTransform))
  (Variables|Default|SetFBSelect "NewEnumerator1")
  (bind _output_get (Variables|Default|SetSpawnableSelect (Utilities|Select :Index (Math|Random|RandomInteger (+ (Utilities|Array|Get(acopy) (Variables|Default|GetObstacleArray) (Variables|Default|GetTimer%20Speed%20Index)) 1)) :Option%200 "NewEnumerator0" :Option%201 "NewEnumerator1" :Option%202 "NewEnumerator2" :Option%203 "NewEnumerator0")))
  (switch Utilities|FlowControl|Switch|SwitchonESpawnableSelect _output_get
    (:NewEnumerator0
      ;[1 1 1] Acorn (1-point Collectible)
      (bind _returnvalue_2 (Game|SpawnActorfromClass "/Game/Blueprints/BP_AcornSpawnable.BP_AcornSpawnable_C" _returnvalue "Undefined" 0 0))
      (Variables|/Game/Blueprints/BP_SpawnableParent.BP_SpawnableParent_C|SetSpeed%20Multiplier _returnvalue_2 (Variables|Default|GetGlobal%20Speed))
      ;[1 1 1] Call Increase Speed every 5 acorns spawned
      (bind _output_get_2 (Variables|Default|SetAcorns%20Thrown%20Count (+ (Variables|Default|GetAcorns%20Thrown%20Count) 1)))
      (if (== (Math|Integer|%(Integer) _output_get_2 5) 0)
        (CallFunction|IncreaseSpeed)
        (Development|PrintString "5th acorn thrown")))
    (:NewEnumerator1
      ;[1 0.02396 0.02396] Tree Branch (Obstacle)
      (bind _returnvalue_3 (Game|SpawnActorfromClass "/Game/Blueprints/BP_TreeBranch.BP_TreeBranch_C" _returnvalue "Undefined" 0 0))
      (Variables|/Game/Blueprints/BP_SpawnableParent.BP_SpawnableParent_C|SetSpeed%20Multiplier _returnvalue_3 (Variables|Default|GetGlobal%20Speed)))
    (:NewEnumerator2
      ;[1 0.02396 0.02396] Nugget (2-point Collectible)
      (bind _returnvalue_4 (Game|SpawnActorfromClass "/Game/Blueprints/BP_SpawnableParent.BP_SpawnableParent_C" _returnvalue "Undefined" 0 0))
      (Variables|/Game/Blueprints/BP_SpawnableParent.BP_SpawnableParent_C|SetSpeed%20Multiplier _returnvalue_4 (Variables|Default|GetGlobal%20Speed)))))

(fn UpdateAnimation
  (Sprite|SetFlipbook (Variables|Default|GetPaperFlipbook%20-%20GirlSquirrel) (Utilities|Select :Index (Variables|Default|GetFBSelect) :NewEnumerator0 (Variables|Flipbooks|GetDigging%20In%20Tree) :NewEnumerator1 (Variables|Flipbooks|GetThrowing%20Spawnable) :NewEnumerator2 (Variables|Flipbooks|GetIdle) :NewEnumerator3 0 :NewEnumerator4 0)))

(fn Movement
  (bind _returnvalue (Transformation|GetActorLocation))
  (bind _max_left_location (Variables|Default|GetMax%20Left%20Location))
  (bind _max_right_location (Variables|Default|GetMax%20Right%20Location))
  (Development|PrintString "Movement Called" true true "(R=0.968215,G=0.258287,B=1.000000,A=1.000000)")
  (if (not (Variables|Default|GetMoving?))
    (Variables|Default|SetMoving? true)
    (Utilities|FlowControl|Sequence
      (:then_0
        (bind _output_get (LocalVariables|SetTarget%20Location (Math|Vector|MakeVector (Math|Random|RandomFloatinRange (.x _max_left_location) (.x _max_right_location)) (Math|Random|RandomFloatinRange (.y _max_left_location) (.y _max_right_location)) 0.0)))
        (Development|PrintString (Utilities|String|ToString(Vector) _output_get) true true "(R=0.862243,G=1.000000,B=0.000000,A=1.000000)"))
      (:then_1
        (LocalVariables|SetMove%20By%20Float (Math|Random|RandomIntegerinRange 150 200))
        (LocalVariables|SetMove%20By (/ (- (LocalVariables|GetTarget%20Location) (Transformation|GetActorLocation)) (Math|Vector|MakeVector (Math|Conversions|ToFloat(Integer) (LocalVariables|GetMove%20By%20Float)) (Math|Conversions|ToFloat(Integer) (LocalVariables|GetMove%20By%20Float)) 0.0)))
        (while (Utilities|Operators|NotEqual(!=) (Math|Vector|MakeVector (.x _returnvalue) (.y _returnvalue) 0.0) (Math|Vector|MakeVector (.x (LocalVariables|GetTarget%20Location)) (.y (LocalVariables|GetTarget%20Location)) 0.0) 2.0)
          ;[1 1 1] Actor Location += Move By incrementor
          (Transformation|SetActorLocation (+ (Transformation|GetActorLocation) (LocalVariables|GetMove%20By)) false false)
          (Development|PrintString "Moved Spawnbox" true true "(R=1.000000,G=0.637919,B=0.026042,A=1.000000)"))
        (Variables|Default|SetMoving? false)
        ;[1 1 1] Delay 3.0-6.0s and call Movement again
        (Utilities|Time|SetTimerbyFunctionName 0 "Movement" 0.0 false 4.5 1.5)))))