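; Tree branch actor that drifts along X toward where the player character stood when the branch began play, until it reaches the ground.
; BeginPlay caches the player's location once, so the branch does not follow later movement.
; Each Tick, TargetedMovement closes a small fixed fraction of the remaining X gap, an ease-out independent of delta time.
; Once GroundCheck passes, movement stops and Disappear runs after a short delay.
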(event EventBeginPlay
  (bind _returnvalue (Actor|GetActorOfClass "/Game/Blueprints/BP_PlayerCharacter.BP_PlayerCharacter_C"))
  (Variables|Default|SetPC_Target (Transformation|GetActorLocation _returnvalue)))

(event Collision|EventActorBeginOverlap
  (params (OtherActor :type Actor%20Object%20Reference)))

(event EventTick
  (params (DeltaSeconds :type Float%20%28single-precision%29))
  (bind _time_to_disappear_ (CallFunction|GroundCheck))
  (if _time_to_disappear_
    (Utilities|FlowControl|Delay 1.0)
    (CallFunction|Disappear)
    (else
      (CallFunction|TargetedMovement))))

(fn ConstructionScript
  (|CallParentFunction))

(fn TargetedMovement
  (bind _returnvalue (Transformation|GetActorLocation))
  (Transformation|SetActorLocationAndRotation (Math|Vector|MakeVector (+ (.x _returnvalue) (/ (- (.x (Variables|Default|GetPC_Target)) (.x _returnvalue)) 2e+02)) 0.0 0.0) (Math|Rotator|MakeRotator 0.0 0.0 0.0)))