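; BP_AcornSpawnable is a falling acorn collectible that awards points when touched, built on a parent spawnable class.
; Construction picks a random target X and a spin direction based on which half of the range it falls in.
; Tick eases X toward that target while falling along Y with a speed multiplier, until the parent's ground check holds it and triggers a delayed Disappear.
; Earlier arc-movement logic remains unconnected.
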(event EventBeginPlay
  ;[1 1 1] Length of time C.Script logic takes
  (Utilities|FlowControl|Delay 1.7)
  (Variables|Default|SetspawnOver? true)
  (Variables|Default|SetDisappear%20FB 0))

(event EventTick
  (params (DeltaSeconds :type Float%20%28single-precision%29))
  (bind _returnvalue (Transformation|GetActorLocation))
  (bind _time_to_disappear_ (CallFunction|GroundCheck))
  (if _time_to_disappear_
    ;[1 1 1] Stop Y movement. Wait for Parent Destruction to be called
    (Transformation|SetActorLocationAndRotation (Math|Vector|MakeVector (.x _returnvalue) (.y _returnvalue) (.z _returnvalue)) (Transformation|GetActorRotation))
    (Utilities|FlowControl|Delay 1.0)
    (CallFunction|Disappear)
    (else
      (CallFunction|Movement (Variables|Default|GetspawnOver?)))))

(fn ConstructionScript
  (|CallParentFunction)
  (Utilities|FlowControl|Sequence
    (:then_0
      ;[1 1 1] Define starting arc, which ends with acorn at a different x-value than SpawnBox
      (Variables|Default|SetXValue (Math|Random|RandomFloatinRange 2.6e+02 6.6e+02)))
    (:then_1
      ;[1 1 1] Define Acorn IS a Collectible (gives points for touching) and set rotation amount (for Flipbook, purely visual)
      (Variables|Default|SetIsCollectible? true)
      (if (<= (Variables|Default|GetXValue) 4.7e+02)
        (Variables|Default|SetRotation (Math|Random|RandomFloatinRange -7.0 0.0))
        (else
          (Variables|Default|SetRotation (Math|Random|RandomFloatinRange 0.0 7.0))))
      (Transformation|AddActorLocalRotation (Math|Rotator|MakeRotator 0.0 0.0 (Variables|Default|GetRotation)) false false))))

(fn NewFunction00)

(fn TouchingPlayerGood
  (params (AddScorePoint :type Integer))
  (|CallParentFunction 0))

(fn LoseLife
  (|CallParentFunction))

(fn TouchingGroundBad
  (params (NewParam :type Integer))
  (|CallParentFunction 0))

(fn TouchingGroundGood
  (|CallParentFunction))

(fn Movement
  (params (Spawn%20Over? :type Boolean))
  (bind _returnvalue (Transformation|GetActorLocation))
  (Transformation|SetActorLocationAndRotation (Math|Vector|MakeVector (+ (.x _returnvalue) (/ (- (Variables|Default|GetXValue) (.x _returnvalue)) 2e+02)) (+ (.y _returnvalue) (+ 2.5 (Variables|Default|GetSpeed%20Multiplier))) 0.0) (Math|Rotator|MakeRotator 0.0 0.0 (+ (.yaw (Transformation|GetActorRotation)) (Variables|Default|GetRotation)))))

(fn GroundCheck
  ;[1 1 1] Check if on Ground every tick
  (bind _time_to_disappear_ (|CallParentFunction))
  (return _time_to_disappear_))