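; Game state Blueprint that tracks level, score and lives and handles the game-over flow.
; BeginPlay starts at the first level with zero score and the configured starting lives.
; The GameOver event waits briefly so falling acorns land, then shows the game-over widget, pauses the game and switches input to game and UI with that widget focused.
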(event Custom|Game%20Over
  (Utilities|FlowControl|Delay 1.5) ; Allow last acorn(s) to fall
  (bind _returnvalue (UserInterface|CreateWidget "/Game/Levels/ui_GameOver.ui_GameOver_C"))
  (UserInterface|Viewport|AddtoViewport _returnvalue 0)
  ;[1 1 1] Pause Game and allow Mouse Input to Game Over screen
  (Game|SetGamePaused true)
  (Input|SetInputModeGameandUI (Game|GetPlayerController 0) _returnvalue "DoNotLock" false false))

(event EventBeginPlay
  (Variables|Default|SetCurrentLevel 1)
  (Variables|Default|SetCurrentScore 0)
  (Variables|Default|SetCurrentLives (Variables|Default|GetStartingLives)))

(event EventTick
  (params (DeltaSeconds :type Float%20%28single-precision%29)))

(fn ConstructionScript)